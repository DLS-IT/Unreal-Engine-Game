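; BP_Doors is an interactable two-panel sliding door that can be locked by a key ID.
; Use toggles the door, moving both cube panels apart or back with timed MoveComponentTo calls and playing a sound.
; When locked, it checks the player's KeyRing, then either unlocks without opening or plays an error buzz.
; The cached BP_Player reference is fetched on BeginPlay and again on PlayerDeath.
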(event `PlayerDeath`
  (`self.GetPlayerREF`))

(event `self.ReceiveBeginPlay`
  (`self.GetPlayerREF`))

(event `GetPlayerREF`
  (bind _asbp_player (cast `/Game/Blueprints/BP_Player` (`GameplayStatics.GetPlayerCharacter` 0)))
  (set `self.PlayerREF` _asbp_player))

(event `/Game/Blueprints/Interface/Use_Interface.Use`
  (`self.ToogleDoor`))

(event `OpenFirstPart`
  ;[1 1 1] First Part (Left Door)
  (`KismetSystemLibrary.MoveComponentTo` (`self.Cube`) (0.0 243.0 200.0) (struct) true true 1.0))

(event `OpenSecondPart`
  ;[1 1 1] Second Part (Right Door)
  (`KismetSystemLibrary.MoveComponentTo` (`self.Cube1`) (0.0 -257.0 200.0) (struct) true true 1.0))

(event `ToogleDoor`
  ;[1 1 1] Close or Open The Door
  (if (`self.Locked`)
    (if (`KismetArrayLibrary.Array_Contains` (`/Game/Blueprints/BP_Player.KeyRing` (`self.PlayerREF`)) (`self.KeyID`))
      (`self.UnlockDoor`)
      (else
        (`GameplayStatics.PlaySound2D` "/Game/Interface_And_Item_Sounds/WAV/Error_Buzz_05.Error_Buzz_05" 1.0 1.0 0.0 null null)))
    (elif (`self.Open`)
      (`self.CloseDoor`)
      (else
        (`self.OpenDoor`)))))

(event `CloseFirstPart`
  ;[1 1 1] First Part (Left Door)
  (`KismetSystemLibrary.MoveComponentTo` (`self.Cube`) (0.0 143.0 200.0) (struct) false false 1.0))

(event `CloseSecondPart`
  ;[1 1 1] Second Part (Right Door)
  (`KismetSystemLibrary.MoveComponentTo` (`self.Cube1`) (0.0 -157.0 200.0) (struct) true true 1.0))

(event `OpenDoor`
  ;[1 1 1] Open/Clsse Event
  (`self.OpenFirstPart`)
  (`self.OpenSecondPart`)
  (set `self.Open` true)
  (`GameplayStatics.PlaySound2D` "/Game/Interface_And_Item_Sounds/WAV/Futuristic_Click_04.Futuristic_Click_04" 1.0 1.0 0.0 null null))

(event `CloseDoor`
  ;[1 1 1] Open/Clsse Event
  (`self.CloseFirstPart`)
  (`self.CloseSecondPart`)
  (set `self.Open` false)
  (`GameplayStatics.PlaySound2D` "/Game/Interface_And_Item_Sounds/WAV/Futuristic_Click_06.Futuristic_Click_06" 1.0 1.0 0.0 null null))

(event `LockDoor`
  (set `self.Locked` true))

(event `UnlockDoor`
  (set `self.Locked` false)
  (`GameplayStatics.PlaySound2D` "/Game/Interface_And_Item_Sounds/WAV/Special_Musical_04.Special_Musical_04" 1.0 1.0 0.0 null null))

(fn `UserConstructionScript`)