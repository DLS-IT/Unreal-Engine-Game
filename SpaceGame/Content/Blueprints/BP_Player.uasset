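; Player character Blueprint handling movement, unlockable jump, camera line-trace interaction through Use_Interface, key ring, keypad and pause menus.
; Score pays for two timed powers: fire resistance and revealing BP_Indice actors.
; Damage updates health through BP_PlayerController, with a looping timer applying fire damage unless resisted.
; Death ragdolls and destroys the pawn, and Destroyed has BP_Gamemode respawn it at the saved transform, carrying jump, keys and score.
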(event `Adding_Key`
  (params (NewItem :type "Name (by ref)"))
  (`KismetArrayLibrary.Array_Add` (`self.KeyRing`) NewItem))

(event `PlayerinFire`
  (`GameplayStatics.ApplyDamage` (`GameplayStatics.GetPlayerCharacter` 0) (* (`KismetMathLibrary.Conv_BoolToDouble` (`self.Damaged_by_Fire`)) 20.0))
  (bind _returnvalue (`KismetSystemLibrary.K2_SetTimer` null "FireDamage" 0.5 true)))

(event `PlayerNotInFire`
  (`KismetSystemLibrary.K2_ClearAndInvalidateTimerHandle` (stale `PlayerinFire` _returnvalue)))

(event `InputAction|Activate Resistance Fire`
  (params (Key :type "Key Structure"))
  (:`Pressed`
    (if (>= (`self.Score`) 10)
      (`GameplayStatics.PlaySound2D` "/Game/Interface_And_Item_Sounds/WAV/Special_Powerup_09.Special_Powerup_09" 1.0 1.0 0.0 null null)
      (`self.UpdateScore` -10)
      (`ActorComponent.Activate` (`self.SFX_BodyPlayer1`) false)
      (set `self.Damaged_by_Fire` false)
      (bind _asbp_player_controller (cast `/Game/Blueprints/BP_PlayerController` (`GameplayStatics.GetPlayerController` 0)))
      (`/Game/Blueprints/BP_PlayerController.Set_Visibility_FireResistance` _asbp_player_controller true)
      (`KismetSystemLibrary.Delay` 5.0)
      (`/Game/Blueprints/BP_PlayerController.Set_Visibility_FireResistance` _asbp_player_controller false)
      (`ActorComponent.Deactivate` (`self.SFX_BodyPlayer1`))
      (set `self.Damaged_by_Fire` true))))

(event `InputAction|Interact`
  (params (Key :type "Key Structure"))
  (:`Pressed`
    (`self.LineTrace`)))

(event `LineTrace`
  (bind _camera (`self.Camera`))
  (bind _returnvalue (`SceneComponent.K2_GetComponentLocation` _camera))
  ;[1 1 1] Interaction
  ;;[1 1 1] Line Trace by channe, using the camera as reference
  (bind (_outhit _returnvalue_2) (`KismetSystemLibrary.LineTraceSingle` _returnvalue (+ _returnvalue (* (`SceneComponent.GetForwardVector` _camera) 400.0)) "TraceTypeQuery1"))
  (if _returnvalue_2
    (bind (_bblockinghit _binitialoverlap _time _distance _location _impactpoint _normal _impactnormal _physmat _hitactor) (`GameplayStatics.BreakHitResult` _outhit))
    (if (`KismetSystemLibrary.DoesImplementInterface` _hitactor "/Game/Blueprints/Interface/Use_Interface.Use_Interface_C")
      (message `/Game/Blueprints/Interface/Use_Interface.Use` _hitactor))))

(event `InputAction|Activate Revelling Indices`
  (params (Key :type "Key Structure"))
  (:`Pressed`
    (if (>= (`self.Score`) 10)
      (`GameplayStatics.PlaySound2D` "/Game/Interface_And_Item_Sounds/WAV/Special_Powerup_03.Special_Powerup_03" 1.0 1.0 0.0 null null)
      (`ActorComponent.Activate` (`self.SFX_SearchIndice`) false)
      (`self.UpdateScore` -10)
      (bind _outactors (`GameplayStatics.GetAllActorsOfClass` "/Game/Blueprints/Actors/BP_Indice.BP_Indice_C"))
      (`/Game/Blueprints/Actors/BP_Indice.Show_Indice` _outactors)
      (`KismetSystemLibrary.Delay` 15.0)
      (bind _outactors_2 (`GameplayStatics.GetAllActorsOfClass` "/Game/Blueprints/Actors/BP_Indice.BP_Indice_C"))
      (`/Game/Blueprints/Actors/BP_Indice.Hide_Indice` _outactors_2)
      (`ActorComponent.Deactivate` (`self.SFX_SearchIndice`)))))

(event `self.ReceiveBeginPlay`
  (set `self.Health` (`self.MaxHealth`))
  (set `self.PlayerRespawnTransform` (`self.GetTransform`))
  (bind _asbp_player_controller (cast `/Game/Blueprints/BP_PlayerController` (`self.GetController`)))
  (`/Game/Blueprints/BP_PlayerController.UpdateHealthBar` _asbp_player_controller (`self.Health`) (`self.MaxHealth`))
  (`self.StartCinematics`))

(event `add_Jump`
  (set `self.can_Jump` true))

(event `Add_KeyRing`
  (params (KeyRing :type "Array of Name"))
  (set `self.KeyRing` KeyRing))

(event `Show_Digicode`
  (params (Code :type String) (DoorKey :type Name))
  (bind _returnvalue (`GameplayStatics.GetPlayerController` 0))
  ;[1 1 1] Keypad
  (bind _returnvalue_2 (`|CreateWidget` "/Game/UI_Menus/Keypad_Menu/Keypad_Menu.Keypad_Menu_C"))
  (`UserWidget.AddToViewport` _returnvalue_2 0)
  (set `PlayerController.bShowMouseCursor` true _returnvalue)
  (`WidgetBlueprintLibrary.SetInputMode_UIOnlyEx` _returnvalue null)
  (`GameplayStatics.SetGamePaused` true)
  (`/Game/UI_Menus/Keypad_Menu/Keypad_Menu.Set_Digicode` _returnvalue_2 Code)
  (`/Game/UI_Menus/Keypad_Menu/Keypad_Menu.SetKey` _returnvalue_2 DoorKey))

(event `InputAction|Digicode`
  (params (Key :type "Key Structure"))
  ;[1 1 1] Keypad
)

(event `InputAction|Jump`
  (params (Key :type "Key Structure"))
  (bind _can_jump (`self.can_Jump`))
  ;[1 1 1] Input: Mouvement
  (:`Pressed`
    (if _can_jump
      (`self.Jump`)))
  (:`Released`
    (if _can_jump
      (`self.StopJumping`))))

(event `InputAxis|Move Foward/Backward`
  (params (AxisValue :type "Float (single-precision)"))
  (bind (_returnvalue_roll _returnvalue_pitch _returnvalue_yaw) (`KismetMathLibrary.BreakRotator` (`self.GetControlRotation`)))
  ;[1 1 1] Input: Mouvement
  (`self.AddMovementInput` (`KismetMathLibrary.GetForwardVector` (`KismetMathLibrary.MakeRotator` 0.0 0.0 _returnvalue_yaw)) AxisValue))

(event `InputAxis|MouseLookUp`
  (params (AxisValue :type "Float (single-precision)"))
  ;[1 1 1] Input: Mouvement
  (`self.AddControllerPitchInput` AxisValue))

(event `InputAction|Pause`
  (params (Key :type "Key Structure"))
  (bind _returnvalue (`GameplayStatics.GetPlayerController` 0))
  ;[1 1 1] Pause the game
  (:`Pressed`
    (bind _returnvalue_2 (`|CreateWidget` "/Game/UI_Menus/PauseMenu/PauseMenu.PauseMenu_C"))
    (`UserWidget.AddToViewport` _returnvalue_2 0)
    (set `PlayerController.bShowMouseCursor` true _returnvalue)
    (`WidgetBlueprintLibrary.SetInputMode_UIOnlyEx` _returnvalue null)
    (`GameplayStatics.SetGamePaused` true)))

(event `InputAxis|Move Right/Left`
  (params (AxisValue :type "Float (single-precision)"))
  (bind (_returnvalue_roll _returnvalue_pitch _returnvalue_yaw) (`KismetMathLibrary.BreakRotator` (`self.GetControlRotation`)))
  ;[1 1 1] Input: Mouvement
  (`self.AddMovementInput` (`KismetMathLibrary.GetRightVector` (`KismetMathLibrary.MakeRotator` 0.0 0.0 _returnvalue_yaw)) AxisValue))

(event `InputAxis|MouseLook`
  (params (AxisValue :type "Float (single-precision)"))
  ;[1 1 1] Input: Mouvement
  (`self.AddControllerYawInput` AxisValue))

(event `self.ReceiveAnyDamage`
  (params (Damage :type "Float (single-precision)") (DamageType :type "DamageType Object Reference") (InstigatedBy :type "Controller Object Reference") (DamageCauser :type "Actor Object Reference"))
  (set `self.Health` (`KismetMathLibrary.FClamp` (- (`self.Health`) Damage) 0.0 (`self.MaxHealth`)))
  (bind _asbp_player_controller (cast `/Game/Blueprints/BP_PlayerController` (`self.GetController`)))
  (`/Game/Blueprints/BP_PlayerController.UpdateHealthBar` _asbp_player_controller (`self.Health`) (`self.MaxHealth`))
  (if (<= (`self.Health`) 0.0)
    (`self.PlayerDeath`)))

(event `Respaw`
  (bind _sfx_respawn (`self.SFX_Respawn`))
  (`ActorComponent.Activate` _sfx_respawn false)
  (`KismetSystemLibrary.Delay` 3.0)
  (`ActorComponent.Deactivate` _sfx_respawn))

(event `SetNewRespawnTransform`
  (params (NewPlayerRespawnTransform :type "Transform Structure"))
  (set `self.PlayerRespawnTransform` NewPlayerRespawnTransform))

(event `UpdateHealth`
  (`self.OnDamaged`))

(event `UpdateScore`
  (params (Score :type Integer))
  (set `self.Score` (+ Score (`self.Score`)))
  (bind _asbp_player_controller (cast `/Game/Blueprints/BP_PlayerController` (`GameplayStatics.GetPlayerController` 0)))
  (`/Game/Blueprints/BP_PlayerController.Set_Score` _asbp_player_controller (`self.Score`)))

(event `PlayerWon`
  (`KismetSystemLibrary.PrintString` "The Playe has finish the game"))

(event `PlayerDeath`
  (`PrimitiveComponent.SetSimulatePhysics` (`self.Mesh`) true)
  (`PrimitiveComponent.SetCollisionEnabled` (`self.Mesh`) "PhysicsOnly")
  (`PrimitiveComponent.SetCollisionEnabled` (`self.CapsuleComponent`) "NoCollision")
  (set `self.Health` 0.0)
  (`CharacterMovementComponent.DisableMovement` (`self.CharacterMovement`))
  (`KismetSystemLibrary.Delay` 3.0)
  (`self.K2_DestroyActor`))

(event `self.ReceiveDestroyed`
  (bind _asbp_gamemode (cast `/Game/Blueprints/BP_Gamemode` (`GameplayStatics.GetGameMode`)))
  (`/Game/Blueprints/BP_Gamemode.Respawn Player` _asbp_gamemode (`self.PlayerRespawnTransform`) (`self.can_Jump`) (`self.KeyRing`) (`self.Score`)))

(fn `FireDamage`
  (if (`self.Damaged_by_Fire`)
    (`GameplayStatics.ApplyDamage` (`GameplayStatics.GetPlayerCharacter` 0) 20.0)))

(fn `UserConstructionScript`)