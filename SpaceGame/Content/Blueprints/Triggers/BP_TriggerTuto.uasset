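; Trigger volume that shows a tutorial widget on screen while something overlaps its box.
; A TriggerBoxType enum selects which widget class to create, covering movement, health, card, reveal, fire, death and jump tutorials.
; Begin overlap creates that widget for the first player controller, stores it and adds it to the viewport; end overlap removes it.
; Neither overlap event filters the overlapping actor.
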(event `self.Box.OnComponentBeginOverlap`
  (params (OverlappedComponent :type "PrimitiveComponent Object Reference") (OtherActor :type "Actor Object Reference") (OtherComp :type "PrimitiveComponent Object Reference") (OtherBodyIndex :type Integer) (bFromSweep :type Boolean) (SweepResult :type "HitResult Structure (by ref)"))
  (bind _returnvalue (`GameplayStatics.GetPlayerController` 0))
  (switch `/Game/Blueprints/Triggers/E_TutoWidget` (`self.TriggerBoxType`)
    (:`NewEnumerator0`
      (bind _returnvalue_2 (`|CreateWidget` "/Game/UI_Menus/Tutos/MovmentTuto.MovmentTuto_C" _returnvalue))
      (bind _output_get (set `self.Tuto` _returnvalue_2))
      (`UserWidget.AddToViewport` _output_get 0))
    (:`NewEnumerator1`
      (bind _returnvalue_3 (`|CreateWidget` "/Game/UI_Menus/Tutos/HealthTuto.HealthTuto_C" _returnvalue))
      (bind _output_get_2 (set `self.Tuto` _returnvalue_3))
      (`UserWidget.AddToViewport` _output_get_2 0))
    (:`NewEnumerator2`
      (bind _returnvalue_4 (`|CreateWidget` "/Game/UI_Menus/Tutos/CardTuto.CardTuto_C" _returnvalue))
      (bind _output_get_3 (set `self.Tuto` _returnvalue_4))
      (`UserWidget.AddToViewport` _output_get_3 0))
    (:`NewEnumerator3`
      (bind _returnvalue_5 (`|CreateWidget` "/Game/UI_Menus/Tutos/RevealTuto.RevealTuto_C" _returnvalue))
      (bind _output_get_4 (set `self.Tuto` _returnvalue_5))
      (`UserWidget.AddToViewport` _output_get_4 0))
    (:`NewEnumerator4`
      (bind _returnvalue_6 (`|CreateWidget` "/Game/UI_Menus/Tutos/FireTuto.FireTuto_C" _returnvalue))
      (bind _output_get_5 (set `self.Tuto` _returnvalue_6))
      (`UserWidget.AddToViewport` _output_get_5 0))
    (:`NewEnumerator5`
      (bind _returnvalue_7 (`|CreateWidget` "/Game/UI_Menus/Tutos/DeathTuto.DeathTuto_C" _returnvalue))
      (bind _output_get_6 (set `self.Tuto` _returnvalue_7))
      (`UserWidget.AddToViewport` _output_get_6 0))
    (:`NewEnumerator6`
      (bind _returnvalue_8 (`|CreateWidget` "/Game/UI_Menus/Tutos/JumpTuto.JumpTuto_C" _returnvalue))
      (bind _output_get_7 (set `self.Tuto` _returnvalue_8))
      (`UserWidget.AddToViewport` _output_get_7 0))))

(event `self.Box.OnComponentEndOverlap`
  (params (OverlappedComponent :type "PrimitiveComponent Object Reference") (OtherActor :type "Actor Object Reference") (OtherComp :type "PrimitiveComponent Object Reference") (OtherBodyIndex :type Integer))
  (`Widget.RemoveFromParent` (`self.Tuto`)))

(fn `UserConstructionScript`)