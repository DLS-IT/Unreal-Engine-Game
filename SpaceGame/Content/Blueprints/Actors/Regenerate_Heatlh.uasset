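; Health pickup actor that heals a BP_Player on overlapping its Box by applying negative damage.
; On pickup it plays a particle burst and sound, then hides the Sphere and disables Box collision instead of destroying itself.
; The Recreate event restores visibility and collision if the pickup was consumed; nothing in this graph calls it.
; BeginPlay caches the Box's world transform, which this graph does not use afterward.
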(event `self.ReceiveBeginPlay`
  (set `self.Transform_RegenerateHealth` (`SceneComponent.K2_GetComponentToWorld` (`self.Box`))))

(event `Recreate`
  (bind _box (`self.Box`))
  (if (== 0 (`PrimitiveComponent.GetCollisionEnabled` _box))
    (`PrimitiveComponent.SetCollisionEnabled` _box "QueryAndPhysics")
    (`SceneComponent.SetHiddenInGame` (`self.Sphere`) false false)))

(event `self.Box.OnComponentBeginOverlap`
  (params (OverlappedComponent :type "PrimitiveComponent Object Reference") (OtherActor :type "Actor Object Reference") (OtherComp :type "PrimitiveComponent Object Reference") (OtherBodyIndex :type Integer) (bFromSweep :type Boolean) (SweepResult :type "HitResult Structure (by ref)"))
  (bind _asbp_player (cast `/Game/Blueprints/BP_Player` OtherActor))
  (`GameplayStatics.ApplyDamage` _asbp_player -50.0)
  (`GameplayStatics.SpawnEmitterAtLocation` "/Game/Realistic_Starter_VFX_Pack_Vol2/Particles/Destruction/P_Destruction_Electric.P_Destruction_Electric" (`self.K2_GetActorLocation`))
  (`GameplayStatics.PlaySound2D` "/Game/Interface_And_Item_Sounds/Cues/Coins_05_Cue.Coins_05_Cue" 1.0 1.0 0.0 null null)
  (`SceneComponent.SetHiddenInGame` (`self.Sphere`) true false)
  (`PrimitiveComponent.SetCollisionEnabled` (`self.Box`) "NoCollision"))

(fn `UserConstructionScript`)