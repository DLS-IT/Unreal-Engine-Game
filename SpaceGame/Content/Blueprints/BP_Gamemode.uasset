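; BP_Gamemode is the game mode that handles player respawning and restores state to the new character.
; RespawnPlayer spawns and possesses a BP_Player at the given transform, resets the health bar, and passes on key ring and score.
; It also tells Regenerate_Heatlh actors to recreate and BP_Doors to react to the death.
; If CanJump is set, it calls AddJump and Respaw on the new player.
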(event `PassKeyRing_and_Score`
  (params (Key_Ring :type "Array of Name") (Score :type Integer))
  (bind _asbp_player (cast `/Game/Blueprints/BP_Player` (`GameplayStatics.GetPlayerCharacter` 0)))
  (`/Game/Blueprints/BP_Player.Add_KeyRing` _asbp_player Key_Ring)
  (set `/Game/Blueprints/BP_Player.Score` Score _asbp_player))

(event `RecreateHealth`
  (bind _outactors (`GameplayStatics.GetAllActorsOfClass` "/Game/Blueprints/Actors/Regenerate_Heatlh.Regenerate_Heatlh_C"))
  (`/Game/Blueprints/Actors/Regenerate_Heatlh.Recreate` _outactors))

(event `UpdateDoor`
  (bind _outactors (`GameplayStatics.GetAllActorsOfClass` "/Game/Blueprints/Interaction/BP_Doors.BP_Doors_C"))
  (`/Game/Blueprints/Interaction/BP_Doors.PlayerDeath` _outactors))

(event `Respawn Player`
  (params (SpawnTransform :type "Transform Structure") (CanJump :type Boolean) (Key_Ring :type "Array of Name (by ref)") (Score :type Integer))
  (bind _returnvalue (`GameplayStatics.GetPlayerController` 0))
  (bind _returnvalue_2 (`|SpawnActorFromClass` "/Game/Blueprints/BP_Player.BP_Player_C" SpawnTransform "Undefined" "MultiplyWithRoot" null null))
  (`Controller.Possess` _returnvalue _returnvalue_2)
  (bind _asbp_player_controller (cast `/Game/Blueprints/BP_PlayerController` _returnvalue))
  (`/Game/Blueprints/BP_PlayerController.UpdateHealthBar` _asbp_player_controller 100.0 100.0)
  (`self.PassKeyRing_and_Score` Key_Ring Score)
  (`self.RecreateHealth`)
  (`self.UpdateDoor`)
  (bind _output_get (set `self.CanJump` CanJump))
  (if _output_get
    (bind _asbp_player (cast `/Game/Blueprints/BP_Player` (`GameplayStatics.GetPlayerCharacter` 0)))
    (`/Game/Blueprints/BP_Player.add_Jump` _asbp_player)
    (`/Game/Blueprints/BP_Player.Respaw` _asbp_player)))

(fn `UserConstructionScript`)